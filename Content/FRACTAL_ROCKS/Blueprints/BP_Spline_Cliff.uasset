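; Spline-driven cliff builder that lays a chosen mesh along a spline as deformed spline mesh sections.
; The construction script splits the spline by SectionLength and adds one component per section, with clamped tangents and an adjustable end offset.
; Alternate sections get about half a turn of extra roll to show the mesh's other side, on top of the spline's own roll.
; Mesh, material, scale, roll and collision are variables; runtime events are unused.
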(event EventBeginPlay)

(event Collision|EventActorBeginOverlap
  (params (OtherActor :type Actor%20Object%20Reference)))

(event EventTick
  (params (DeltaSeconds :type Float%20%28single-precision%29)))

(fn ConstructionScript
  (bind _scale (Variables|Default|Getscale))
  (bind _roll (Variables|Default|Getroll))
  (bind _scale_2 (Variables|Default|Getscale))
  (bind _roll_2 (Variables|Default|Getroll))
  (bind _material (Variables|Default|Getmaterial))
  (bind _section_length (Variables|Default|GetSection%20Length))
  (bind _spline (Variables|Default|GetSpline))
  (bind _mesh (Variables|Default|GetMesh))
  (bind _returnvalue (+ _roll 3.2))
  ;[1 1 1] Comment
  (for _index (range 0 (Math|Float|Truncate (/ (Spline|GetSplineLength (Variables|Default|GetSpline)) (Variables|Default|GetSection%20Length))))
    ;[1 1 1] create a switch to alternate sides
    (if (> (.Remainder (Math|Float|Division(WholeandRemainder) (Math|Conversions|ToFloat(Integer) _index) 2.0)) 0.0)
      ;[1 1 1] odd iterations , rotation to use the other side
      (bind _returnvalue_2 (AddComponent|AddSplineMeshComponent false))
      (Components|StaticMesh|SetStaticMesh _returnvalue_2 _mesh)
      (Rendering|Material|SetMaterial _returnvalue_2 0 _material)
      (SplineMesh|SetStartandEnd _returnvalue_2 (Spline|GetLocationatDistanceAlongSpline _spline (* _index _section_length) "Local") (Math|Vector|ClampVectorSize (Spline|GetTangentatDistanceAlongSpline _spline (* _index _section_length) "Local") 0.0 _section_length) (Spline|GetLocationatDistanceAlongSpline _spline (+ (* (+ _index 1) _section_length) (Variables|Default|Getend%20offset)) "Local") (Math|Vector|ClampVectorSize (Spline|GetTangentatDistanceAlongSpline _spline (+ (* (+ _index 1) _section_length) (Variables|Default|Getend%20offset)) "Local") 0.0 _section_length) true :!class /Script/Engine.SplineMeshComponent)
      (Class|SplineMeshComponent|SetStartRoll _returnvalue_2 (+ _returnvalue (/ (.Roll (Math|Rotator|BreakRotator (Spline|GetRotationatDistanceAlongSpline (Variables|Default|GetSpline) (* _index _section_length) "Local"))) 1e+02)) true)
      (Class|SplineMeshComponent|SetEndRoll _returnvalue_2 (+ _returnvalue (/ (.Roll (Math|Rotator|BreakRotator (Spline|GetRotationatDistanceAlongSpline (Variables|Default|GetSpline) (+ (* (+ _index 1) _section_length) (Variables|Default|Getend%20offset)) "Local"))) 1e+02)) true)
      (SplineMesh|SetStartScale _returnvalue_2 _scale true :!class /Script/Engine.SplineMeshComponent)
      (SplineMesh|SetEndScale _returnvalue_2 _scale true :!class /Script/Engine.SplineMeshComponent)
      (SplineMesh|SetEndOffset _returnvalue_2 (Variables|Default|Getenf%20offset%20alignements) true)
      (Collision|SetCollisionEnabled _returnvalue_2 (Variables|Default|GetCollisions%20?))
      (else
        ;[1 1 1] even iterations
        (bind _returnvalue_3 (AddComponent|AddSplineMeshComponent false))
        (Components|StaticMesh|SetStaticMesh _returnvalue_3 _mesh)
        (Rendering|Material|SetMaterial _returnvalue_3 0 _material)
        (SplineMesh|SetStartandEnd _returnvalue_3 (Spline|GetLocationatDistanceAlongSpline _spline (* _index _section_length) "Local") (Math|Vector|ClampVectorSize (Spline|GetTangentatDistanceAlongSpline _spline (* _index _section_length) "Local") 0.0 _section_length) (Spline|GetLocationatDistanceAlongSpline _spline (+ (* (+ _index 1) _section_length) (Variables|Default|Getend%20offset)) "Local") (Math|Vector|ClampVectorSize (Spline|GetTangentatDistanceAlongSpline _spline (+ (* (+ _index 1) _section_length) (Variables|Default|Getend%20offset)) "Local") 0.0 _section_length) true :!class /Script/Engine.SplineMeshComponent)
        (Class|SplineMeshComponent|SetStartRoll _returnvalue_3 (+ _roll_2 (/ (.Roll (Math|Rotator|BreakRotator (Spline|GetRotationatDistanceAlongSpline (Variables|Default|GetSpline) (* _index _section_length) "Local"))) 1e+02)) true)
        (Class|SplineMeshComponent|SetEndRoll _returnvalue_3 (+ _roll_2 (/ (.Roll (Math|Rotator|BreakRotator (Spline|GetRotationatDistanceAlongSpline (Variables|Default|GetSpline) (+ (* (+ _index 1) _section_length) (Variables|Default|Getend%20offset)) "Local"))) 1e+02)) true)
        (SplineMesh|SetStartScale _returnvalue_3 _scale_2 true :!class /Script/Engine.SplineMeshComponent)
        (SplineMesh|SetEndScale _returnvalue_3 _scale_2 true :!class /Script/Engine.SplineMeshComponent)
        (SplineMesh|SetEndOffset _returnvalue_3 (Variables|Default|Getenf%20offset%20alignements) true)
        (Collision|SetCollisionEnabled _returnvalue_3 (Variables|Default|GetCollisions%20?))))))
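; Explosive projectile actor that detonates on a timer, with no impact handling in its graphs.
; The construction script sets the projectile movement's initial speed from the Impulso variable.
; On BeginPlay it waits TimeDilay seconds, then applies radial damage with falloff at its current location, spawns an explosion sound and destruction particle effect there, and destroys itself.
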(event EventBeginPlay
  (Utilities|FlowControl|Delay (Variables|Default|GetTime_dilay))
  (bind _output_get (Variables|Default|SetLocalizacion (Transformation|GetActorLocation)))
  (Class|GameplayStatics|ApplyRadialDamagewithFalloff 1.5e+02 2e+01 _output_get 0.0 1e+03 0.5 0 0 self 0 "ECC_Visibility")
  (Audio|SpawnSoundatLocation "/Game/StarterContent/Audio/Explosion02.Explosion02" (Variables|Default|GetLocalizacion) "0, 0, 0" 1.0 1.0 0.0 0 0)
  (Effects|SpawnEmitteratLocation "/Game/Explosions/Particles/P_Destruction1.P_Destruction1" (Variables|Default|GetLocalizacion) "0, 0, 0" "2.000000,2.000000,2.000000")
  (Actor|DestroyActor))

(fn ConstructionScript
  (Variables|/Script/Engine.ProjectileMovementComponent|SetInitialSpeed (Variables|Default|GetProjectileMovement) (Variables|Default|GetImpulso)))